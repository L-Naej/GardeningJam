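; Game instance for HarvestMoon that builds the level list and handles progression from one level to the next.
; On Init, it queries the Asset Registry for assets directly under /Game/Maps/Levels and keeps the World assets, so levels are discovered without a hand-maintained list.
; LoadNextLevel increments the current index and, if the list entry is valid, opens that map by a name built from its package path and asset name.
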(event Custom|LoadNextLevel
  ;[1 1 1] Load next level logic
  (bind _result (Math|Integer|IncrementInt (Variables|Default|GetCurrentLevelIndex))
    (:%20%20
      (if (Class|AssetRegistryHelpers|IsValid (Utilities|Array|Get(acopy) (Variables|Default|GetLevelsList) _result))
        (Game|OpenLevel(byName) (Utilities|String|StringToName (Utilities|String|Append (Utilities|String|Append (Utilities|String|ToString(Name) (.PackagePath (Utilities|Struct|BreakAssetData (Utilities|Array|Get(acopy) (Variables|Default|GetLevelsList) _result)))) "/") (Utilities|String|ToString(Name) (.AssetName (Utilities|Struct|BreakAssetData (Utilities|Array|Get(acopy) (Variables|Default|GetLevelsList) _result)))))))))))

(event EventInit
  ;[1 1 1] Game initialization
  (for _array_element (.OutAssetData (Class|AssetRegistry|GetAssetsbyPath (Class|AssetRegistryHelpers|GetAssetRegistry) "/Game/Maps/Levels" false false))
    (if (== (Class|AssetRegistryHelpers|GetClass _array_element) "/Script/Engine.World")
      (Utilities|Array|Add (Variables|Default|GetLevelsList) _array_element))))