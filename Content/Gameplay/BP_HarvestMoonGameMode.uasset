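; Game mode for Harvest Moon that configures each level and ends the timed round with a win or lose result.
; Construction script and BeginPlay both read the level-named data table row for time limit and customer settings, appending to the spawn list each time.
; Player restart starts the round timer.
; On expiry, it compares player score to ScoreToWin, triggers the controller's game over and pauses.
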(event Custom|OnRoundEnd
  (bind _asbp_harvest_moon_player_controller (Utilities|Casting|CastToBP_HarvestMoonPlayerController (Game|GetPlayerController 0)))
  (bind _asbp_harvest_moon_player_state (Utilities|Casting|CastToBP_HarvestMoonPlayerState (Variables|/Script/Engine.Controller|GetPlayerState _asbp_harvest_moon_player_controller)))
  (Default|ActivateGameOver _asbp_harvest_moon_player_controller (>= (Variables|/Game/Gameplay/Player/BP_HarvestMoonPlayerState.BP_HarvestMoonPlayerState_C|GetPlayerScore _asbp_harvest_moon_player_state) (Variables|Default|GetScoreToWin)))
  (Game|SetGamePaused true))

(event EventBeginPlay
  (|CallParentFunction)
  (Development|PrintString "GAMEMODEBEGINPLAY")
  ;[1 1 1] Load level data
  (bind _returnvalue (Game|GetCurrentLevelName true))
  (bind _returnvalue_2 (Utilities|GetDataTableRow (Variables|Default|GetLevelsData) (Utilities|String|StringToName _returnvalue))
    (:then
      (Variables|Default|SetRoundDurationInSeconds (.TimeLimitInSeconds (Utilities|Struct|BreakLevelData _returnvalue_2)))
      (Variables|Default|SetNumberOfCustomersToServeToWin (.NumberOfCustomersToServeToWin (Utilities|Struct|BreakLevelData _returnvalue_2)))
      (Variables|Default|SetMaxCustomersToSpawn (.MaxCustomersToSpawn (Utilities|Struct|BreakLevelData _returnvalue_2)))
      (Utilities|Array|AppendArray (Variables|Default|GetCustomersToSpawn) (.CustomersToSpawn (Utilities|Struct|BreakLevelData _returnvalue_2))))
    (:RowNotFound
      (Development|PrintString "Warning: no level data found, falling back to default values." true true "(R=1.000000,G=0.072805,B=0.000000,A=1.000000)"))))

(event EventOnRestartPlayer
  (params (NewPlayer :type Controller%20Object%20Reference))
  (if (> (Variables|Default|GetRoundDurationInSeconds) 0.0)
    (Utilities|Time|SetTimerbyEvent (delegate Custom|OnRoundEnd) (Variables|Default|GetRoundDurationInSeconds))))

(fn ConstructionScript
  (|CallParentFunction)
  (Development|PrintString "GAMEMODE CONSTRUCT SCRIPT")
  ;[1 1 1] Load level data
  (bind _returnvalue (Game|GetCurrentLevelName true))
  (bind _returnvalue_2 (Utilities|GetDataTableRow (Variables|Default|GetLevelsData) (Utilities|String|StringToName _returnvalue))
    (:then
      (Variables|Default|SetRoundDurationInSeconds (.TimeLimitInSeconds (Utilities|Struct|BreakLevelData _returnvalue_2)))
      (Variables|Default|SetNumberOfCustomersToServeToWin (.NumberOfCustomersToServeToWin (Utilities|Struct|BreakLevelData _returnvalue_2)))
      (Variables|Default|SetMaxCustomersToSpawn (.MaxCustomersToSpawn (Utilities|Struct|BreakLevelData _returnvalue_2)))
      (Utilities|Array|AppendArray (Variables|Default|GetCustomersToSpawn) (.CustomersToSpawn (Utilities|Struct|BreakLevelData _returnvalue_2))))
    (:RowNotFound
      (Development|PrintString "Warning: no level data found, falling back to default values." true true "(R=1.000000,G=0.072805,B=0.000000,A=1.000000)"))))