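; BP_Interactable is a clickable or touchable actor, apparently a base class, with an empty OnInteract hook for its interaction.
; A sphere, sized in meters by the construction script, tracks whether the TopDownCharacter is in range.
; Clicks register the actor with BP_HarvestMoonPlayerController and interact immediately if in range.
; Otherwise, overlapping later triggers OnInteract if it is still the last clicked actor, then deactivates the sphere.
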(event OnInputTouchBegin(StaticMesh)
  (params (FingerIndex :type ETouchIndex%20Enum :default "Touch1") (TouchedComponent :type Primitive%20Component%20Object%20Reference))
  ;[1 1 1] If player is too far, it will be used to do the action later when she is close enough.
  (bind _asbp_harvest_moon_player_controller (Utilities|Casting|CastToBP_HarvestMoonPlayerController (Game|GetPlayerController 0)))
  (Default|TrytoRegisterasLastActorClicked _asbp_harvest_moon_player_controller self)
  ;[1 1 1] Player has to be close enough to be able to pick the seed
  (if (Variables|Default|GetbIsPlayerNearEnoughToInteract)
    (CallFunction|OnInteract)))

(event OnComponentBeginOverlap(Sphere)
  (params (OverlappedComponent :type Primitive%20Component%20Object%20Reference) (OtherActor :type Actor%20Object%20Reference) (OtherComp :type Primitive%20Component%20Object%20Reference) (OtherBodyIndex :type Integer) (bFromSweep :type Boolean) (SweepResult :type Hit%20Result%20Structure%20%28by%20ref%29))
  (bind _astop_down_character (Utilities|Casting|CastToTopDownCharacter OtherActor))
  (Variables|Default|SetbIsPlayerNearEnoughToInteract true)
  (bind _asbp_harvest_moon_player_controller (Utilities|Casting|CastToBP_HarvestMoonPlayerController (Pawn|GetController _astop_down_character)))
  (bind _result (Default|OverlappedActorIsLastActorClicked _asbp_harvest_moon_player_controller self))
  (if _result
    (CallFunction|OnInteract)
    (Components|Activation|Deactivate (Variables|Default|GetSphere))))

(event OnClicked(StaticMesh)
  (params (TouchedComponent :type Primitive%20Component%20Object%20Reference) (ButtonPressed :type Key%20Structure))
  ;[1 1 1] If player is too far, it will be used to do the action later when she is close enough.
  (bind _asbp_harvest_moon_player_controller (Utilities|Casting|CastToBP_HarvestMoonPlayerController (Game|GetPlayerController 0)))
  (Default|TrytoRegisterasLastActorClicked _asbp_harvest_moon_player_controller self)
  ;[1 1 1] Player has to be close enough to be able to pick the seed
  (if (Variables|Default|GetbIsPlayerNearEnoughToInteract)
    (CallFunction|OnInteract)))

(event OnComponentEndOverlap(Sphere)
  (params (OverlappedComponent :type Primitive%20Component%20Object%20Reference) (OtherActor :type Actor%20Object%20Reference) (OtherComp :type Primitive%20Component%20Object%20Reference) (OtherBodyIndex :type Integer))
  (Utilities|Casting|CastToTopDownCharacter OtherActor)
  (Variables|Default|SetbIsPlayerNearEnoughToInteract false))

(fn ConstructionScript
  (Components|Sphere|SetSphereRadius (Variables|Default|GetSphere) (* (Variables|Configuration|GetPickUpRadiusInMeters) 1e+02) true))

(fn OnInteract)