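; BP_FieldBase is a field actor that assembles a row of BP_FieldColumn child actors in its construction script.
; It spawns the first column, then reads that column's X bounds extent (a half-size) as the spacing step.
; A loop adds the remaining columns up to NbColumns, offsets each along relative X, attaches it to the root and prints its location.
; The event graph has no active logic.
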(event EventBeginPlay)

(event Collision|EventActorBeginOverlap
  (params (OtherActor :type Actor%20Object%20Reference)))

(event EventTick
  (params (DeltaSeconds :type Float%20%28single-precision%29)))

(fn ConstructionScript
  (bind _returnvalue (AddComponent|AddChildActorComponent false))
  (ChildActorComponent|SetChildActorClass _returnvalue "/Game/Gameplay/Fields/BP_FieldColumn.BP_FieldColumn_C")
  (Transformation|AttachComponentToComponent (Variables|/Script/Engine.ChildActorComponent|GetChildActor _returnvalue) (Variables|Default|GetDefaultSceneRoot) "None" "KeepWorld" "KeepWorld" "KeepRelative" false)
  (LocalVariables|SetOrigin (Transformation|GetActorLocation))
  (LocalVariables|SetXDelta (.x (.BoxExtent (Collision|GetActorBounds (Variables|/Script/Engine.ChildActorComponent|GetChildActor _returnvalue) false))))
  (for _index (range 2 (Variables|Configuration|GetNbColumns))
    (bind _returnvalue_2 (AddComponent|AddChildActorComponent true (Math|Transform|MakeTransform (Math|Vector|MakeVector (* (- _index 1) (LocalVariables|GetXDelta)) 0.0 0.0) "0, 0, 0" "1,1,1")))
    (ChildActorComponent|SetChildActorClass _returnvalue_2 "/Game/Gameplay/Fields/BP_FieldColumn.BP_FieldColumn_C")
    (Transformation|SetActorRelativeLocation (Variables|/Script/Engine.ChildActorComponent|GetChildActor _returnvalue_2) (Math|Vector|MakeVector (* (- _index 1) (LocalVariables|GetXDelta)) 0.0 0.0))
    (Transformation|AttachComponentToComponent (Variables|/Script/Engine.ChildActorComponent|GetChildActor _returnvalue_2) (Variables|Default|GetDefaultSceneRoot) "None" "KeepRelative" "KeepRelative" "KeepRelative" false)
    (Development|PrintString (Utilities|String|ToString(Vector) (Transformation|GetActorLocation (Variables|/Script/Engine.ChildActorComponent|GetChildActor _returnvalue_2))))))