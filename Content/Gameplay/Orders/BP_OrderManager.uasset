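; Order manager Blueprint that releases timed orders in sequence from the OrdersData table.
; OnNewOrder prints and broadcasts the stored order type, then loads the row at CurrentRow and re-arms a one-shot timer on itself using that row's spawn time.
; The chain stops when no row is found, and nothing in this graph makes the first call.
; BeginPlay binds OnOrderProcessed to OrderHandler, but that event is empty.
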(event Custom|OnNewOrder
  (Development|PrintString (Utilities|String|EnumtoString (Variables|Internal|GetNextOrderType)))
  (Default|CallOnNewOrderDelegate (Variables|Internal|GetNextOrderType))
  (bind _returnvalue (Utilities|GetDataTableRow (Variables|Configuration|GetOrdersData) (Utilities|String|StringToName (Utilities|String|ToString(Integer) (Variables|Internal|GetCurrentRow))))
    (:then
      (Variables|Internal|SetNextOrderType (.Type (Utilities|Struct|BreakOrder _returnvalue)))
      (Utilities|Time|SetTimerbyEvent (delegate Custom|OnNewOrder) (.SpawnTimeInSeconds (Utilities|Struct|BreakOrder _returnvalue)))
      (Math|Integer|IncrementInt (Variables|Internal|GetCurrentRow)))))

(event Custom|OnOrderProcessed
  (params (OrderType :type E_VegetableType%20Enum :default "NewEnumerator0")))

(event EventBeginPlay
  (EventDispatchers|AssignOnOrderProcessed (Variables|Configuration|GetOrderHandler) (delegate Custom|OnOrderProcessed)))

(fn ConstructionScript)