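; Customer spawner that places BP_Customer_Base actors at free BP_CustomerStartLocation points in the level, up to the game mode's maximum.
; BeginPlay caches the limit, vegetable list and spawn points; StartSpawningCustomers spawns immediately, then runs a looping timer until the limit is reached.
; Each customer receives the vegetable list and its start location as Owner, and that location is marked Occupied.
; Reset events zero the count and stop the timer.
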(event Custom|SpawnCustomer
  (if (< (Variables|Internal|GetNumberOfAlreadySpawnedCustomers) (Variables|Config|GetNumberOfCustomersToSpawn))
    ;[1 1 1] Spawn new customer
    (Development|PrintString "Attempt to spawn new customer...")
    (bind (_spawnpointfound _success) (CallFunction|FindFreeSpawnPoint (Variables|Internal|GetCustomerSpawnPoints)))
    (if _success
      (Game|SpawnActorfromClass "/Game/Gameplay/Orders/Customers/BP_Customer_Base.BP_Customer_Base_C" (Transformation|GetActorTransform _spawnpointfound) "AlwaysSpawn" _spawnpointfound "NewEnumerator0" (Variables|Config|GetAvailableVegetablesInLevel) 0)
      (Variables|/Game/Gameplay/Orders/Customers/BP_CustomerStartLocation.BP_CustomerStartLocation_C|SetOccupied _spawnpointfound true)
      (Math|Integer|IncrementInt (Variables|Internal|GetNumberOfAlreadySpawnedCustomers)))
    (else
      (Utilities|Time|ClearandInvalidateTimerbyHandle (Variables|Internal|GetSpawnTimerHandle)))))

(event Custom|StartSpawningCustomers
  (Development|PrintString "StartSpawningCustomers")
  (CallFunction|SpawnCustomer) ; First spawn before starting timer
  (Math|Integer|IncrementInt (Variables|Internal|GetNumberOfAlreadySpawnedCustomers)
    (:%20%20
      (bind _returnvalue (Utilities|Time|SetTimerbyEvent (delegate Custom|SpawnCustomer) (Variables|Config|GetNumberOfSecondsBetweenSpawns) true))
      (Variables|Internal|SetSpawnTimerHandle _returnvalue))))

(event EventBeginPlay
  ;[1 1 1] Load data from gamemode
  (bind _asbp_harvest_moon_game_mode (Utilities|Casting|CastToBP_HarvestMoonGameMode (Game|GetGameMode))
    (:then
      (Variables|Config|SetNumberOfCustomersToSpawn (Variables|/Game/Gameplay/BP_HarvestMoonGameMode.BP_HarvestMoonGameMode_C|GetMaxCustomersToSpawn _asbp_harvest_moon_game_mode))
      (Utilities|Array|AppendArray (Variables|Config|GetCustomersToSpawn) (Variables|/Game/Gameplay/BP_HarvestMoonGameMode.BP_HarvestMoonGameMode_C|GetCustomersToSpawn _asbp_harvest_moon_game_mode))
      (Utilities|Array|AppendArray (Variables|Config|GetAvailableVegetablesInLevel) (Variables|/Game/Gameplay/BP_HarvestMoonGameMode.BP_HarvestMoonGameMode_C|GetAvailableVegetables _asbp_harvest_moon_game_mode))
      ;;[1 1 1] Gather customer spawn points from the current level
      (bind _outactors (Actor|GetAllActorsOfClass "/Game/Gameplay/Orders/Customers/BP_CustomerStartLocation.BP_CustomerStartLocation_C"))
      (Utilities|Array|AppendArray (Variables|Internal|GetCustomerSpawnPoints) _outactors))
    (:CastFailed
      (Development|PrintString "Failed to cast game mode"))))

(event EventOnResetLevel
  (Development|PrintString "Reset customer spawner")
  ;[1 1 1] Reinit and clear some internal data on reset.
  (Variables|Internal|SetNumberOfAlreadySpawnedCustomers 0)
  (Utilities|Time|ClearandInvalidateTimerbyHandle (Variables|Internal|GetSpawnTimerHandle)))

(event EventOnReset
  (Development|PrintString "Reset customer spawner")
  ;[1 1 1] Reinit and clear some internal data on reset.
  (Variables|Internal|SetNumberOfAlreadySpawnedCustomers 0)
  (Utilities|Time|ClearandInvalidateTimerbyHandle (Variables|Internal|GetSpawnTimerHandle)))

(fn ConstructionScript)

(fn FindFreeSpawnPoint
  (params (SpawnPoints :type Array%20of%20BP%20Customer%20Start%20Location%20Object%20References))
  (bind _array_element (Utilities|Array|ForEachLoopwithBreak SpawnPoints :!label _label)
    (:LoopBody
      (if (not (Variables|/Game/Gameplay/Orders/Customers/BP_CustomerStartLocation.BP_CustomerStartLocation_C|GetOccupied _array_element))
        (LocalVariables|SetFreeSpawnPoint _array_element)
        (goto _label Break)))
    (:Completed
      (return (LocalVariables|GetFreeSpawnPoint) (Utilities|IsValid (LocalVariables|GetFreeSpawnPoint))))))