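; Base customer actor that waits at a start location for a vegetable order, then leaves when served or timed out, freeing its spot.
; Init loads per-type stats from a data table and builds a random order from vegetables the level allows, shown as grouped sprites.
; Clicking or touching it registers with the player controller, delivering carried vegetables once the player is in range.
; GiveOrderPart removes delivered items and completes the order when empty.
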(event OnClicked(CapsuleComponent)
  (params (TouchedComponent :type Primitive%20Component%20Object%20Reference) (ButtonPressed :type Key%20Structure))
  (bind _asbp_harvest_moon_player_controller (Utilities|Casting|CastToBP_HarvestMoonPlayerController (Game|GetPlayerController 0)))
  (Default|TrytoRegisterasLastActorClicked _asbp_harvest_moon_player_controller self)
  (if (Variables|Default|GetbIsPlayerNearEnoughToInteract)
    (bind _asbp_harvest_moon_player_controller_2 (Utilities|Casting|CastToBP_HarvestMoonPlayerController (Game|GetPlayerController 0)))
    (Default|DeliverCarriedVegetable _asbp_harvest_moon_player_controller_2 self)))

(event OnInputTouchBegin(CapsuleComponent)
  (params (FingerIndex :type ETouchIndex%20Enum :default "Touch1") (TouchedComponent :type Primitive%20Component%20Object%20Reference))
  (bind _asbp_harvest_moon_player_controller (Utilities|Casting|CastToBP_HarvestMoonPlayerController (Game|GetPlayerController 0)))
  (Default|TrytoRegisterasLastActorClicked _asbp_harvest_moon_player_controller self)
  (if (Variables|Default|GetbIsPlayerNearEnoughToInteract)
    (bind _asbp_harvest_moon_player_controller_2 (Utilities|Casting|CastToBP_HarvestMoonPlayerController (Game|GetPlayerController 0)))
    (Default|DeliverCarriedVegetable _asbp_harvest_moon_player_controller_2 self)))

(event OnComponentBeginOverlap(PlayerDetection)
  (params (OverlappedComponent :type Primitive%20Component%20Object%20Reference) (OtherActor :type Actor%20Object%20Reference) (OtherComp :type Primitive%20Component%20Object%20Reference) (OtherBodyIndex :type Integer) (bFromSweep :type Boolean) (SweepResult :type Hit%20Result%20Structure%20%28by%20ref%29))
  (Utilities|Casting|CastToTopDownCharacter OtherActor)
  (Variables|Default|SetbIsPlayerNearEnoughToInteract true)
  (bind _asbp_harvest_moon_player_controller (Utilities|Casting|CastToBP_HarvestMoonPlayerController (Game|GetPlayerController 0)))
  (bind _result (Default|OverlappedActorIsLastActorClicked _asbp_harvest_moon_player_controller self))
  (if _result
    (bind _asbp_harvest_moon_player_controller_2 (Utilities|Casting|CastToBP_HarvestMoonPlayerController (Game|GetPlayerController 0)))
    (Default|DeliverCarriedVegetable _asbp_harvest_moon_player_controller_2 self)))

(event OnComponentEndOverlap(PlayerDetection)
  (params (OverlappedComponent :type Primitive%20Component%20Object%20Reference) (OtherActor :type Actor%20Object%20Reference) (OtherComp :type Primitive%20Component%20Object%20Reference) (OtherBodyIndex :type Integer))
  (Utilities|Casting|CastToTopDownCharacter OtherActor)
  (Variables|Default|SetbIsPlayerNearEnoughToInteract false))

(event Custom|OnCustomerWaitedEnough
  ;[1 1 1] Start waiting timer
  (CallFunction|OnCustomerSatisfied) ; Currently on customer satisfied does the same thing we would like to do here (get out of the map and destroy).
)

(event Custom|OnCustomerSatisfied
  ;[1 1 1] Leave the map when satisfied
  (bind _asbp_customer_start_location (Utilities|Casting|CastToBP_CustomerStartLocation (Components|GetOwner))
    (:then
      (Variables|/Game/Gameplay/Orders/Customers/BP_CustomerStartLocation.BP_CustomerStartLocation_C|SetOccupied _asbp_customer_start_location false))
    (:CastFailed
      _))
  (Actor|DestroyActor))

(event EventBeginPlay
  (CallFunction|Init)
  ;[1 1 1] Start waiting timer
  (Utilities|Time|SetTimerbyEvent (delegate Custom|OnCustomerWaitedEnough) (Variables|Configuration|GetWaitingTimeInSeconds)))

(event EventOnReset
  ;[1 1 1] Customer does not survive the reset event
  (Actor|DestroyActor))

(fn ConstructionScript)

(fn GiveOrderPart
  (params (OrderPart :type E_VegetableType%20Enum :default "NewEnumerator0"))
  (bind _checklist (Variables|Default|GetCheckList))
  (bind _returnvalue (Utilities|Array|FindItem _checklist OrderPart))
  ;[1 1 1] Check the call is valid
  (if (!= _returnvalue -1)
    (bind _output_get (LocalVariables|SetOrderPartIndex _returnvalue))
    (Utilities|Array|RemoveIndex (Variables|Default|GetCheckList) _output_get)
    (Class|PaperGroupedSpriteComponent|RemoveInstance (Variables|Default|GetPaperGroupedSprite) (LocalVariables|GetOrderPartIndex))
    (if (<= (Utilities|Array|Length (Variables|Default|GetCheckList)) 0)
      (CallFunction|OnCustomerSatisfied)
      (return true)
      (else
        (return true)))
    (else
      (Development|PrintString (Utilities|String|Append (Utilities|GetDisplayName self) "Trying to remove an order i did not made!"))
      (return false))))

(fn Init
  ;[1 1 1] Load data depending on customer type
  (bind _returnvalue (Utilities|GetDataTableRow (Variables|Configuration|GetCustomerData) (Utilities|Select :Index (Variables|Configuration|GetType) :NewEnumerator0 "VeggieIn" :NewEnumerator1 "GrandMa" :NewEnumerator2 "BigDistrib"))
    (:then
      (Variables|Configuration|SetWaitingTimeInSeconds (.WaitingTimeInSeconds (Utilities|Struct|BreakCustomerData _returnvalue)))
      (Variables|Configuration|SetMaxItemsNumber (.MaxItemsNumber (Utilities|Struct|BreakCustomerData _returnvalue)))
      (CallFunction|InitCheckListPossibilities (.CheckList (Utilities|Struct|BreakCustomerData _returnvalue)) (Variables|Configuration|GetLevelCheckList))
      (Variables|Configuration|SetTip (.Tip (Utilities|Struct|BreakCustomerData _returnvalue)))
      (Variables|Configuration|SetEcologyRating (.EcologyRating (Utilities|Struct|BreakCustomerData _returnvalue)))
      ;[1 1 1] Greyboxing: display customer type
      (Rendering|Components|TextRender|SetText (Variables|Default|GetTextRender) (Utilities|Text|ToText(String) (Utilities|String|EnumtoString (Variables|Configuration|GetType))))
      ;[1 1 1] Populate checklist based on checklist possibilities from customer data
      (for _index (range 1 (Math|Integer|Clamp(Integer) (Math|Random|RandomInteger (Variables|Configuration|GetMaxItemsNumber)) 1 (Variables|Configuration|GetMaxItemsNumber)))
        (Utilities|Array|Add (Variables|Default|GetCheckList) (Utilities|Array|Get(acopy) (Variables|Configuration|GetCheckListPossibilities) (Math|Random|RandomInteger (Utilities|Array|Length (Variables|Configuration|GetCheckListPossibilities))))))
      ;[1 1 1] Display checklist visually in game
      (for (_array_element _array_index) (Variables|Default|GetCheckList)
        (Utilities|FlowControl|Sequence
          (:then_0
            (switch Utilities|FlowControl|Switch|SwitchonE_VegetableType _array_element
              (:NewEnumerator0
                (LocalVariables|SetOrderSprite "/Game/KenneySpritePack/Items/gemRed_Sprite.gemRed_Sprite"))
              (:NewEnumerator1
                (LocalVariables|SetOrderSprite "/Game/KenneySpritePack/Items/gemGreen_Sprite.gemGreen_Sprite"))
              (:NewEnumerator2
                (LocalVariables|SetOrderSprite "/Game/KenneySpritePack/Items/gemBlue_Sprite.gemBlue_Sprite"))))
          (:then_1
            (Components|InstancedStaticMesh|AddInstance (Variables|Default|GetPaperGroupedSprite) (Math|Transform|MakeTransform (Math|Vector|MakeVector (* (- _array_index (/ (Variables|Configuration|GetMaxItemsNumber) (LocalVariables|GetOrderPartSpriteCenteringOffsetDivider))) 7e+01) 1.0 0.0)) (LocalVariables|GetOrderSprite))))))
    (:RowNotFound
      (Development|PrintString "Warning: no data found for customer" true true "(R=1.000000,G=0.204806,B=0.000000,A=1.000000)"))))

(fn InitCheckListPossibilities
  (params (CustomerTheoreticalCheckList :type Array%20of%20E_VegetableType%20Enums :default "NewEnumerator0") (LevelCheckList :type Array%20of%20E_VegetableType%20Enums :default "NewEnumerator0"))
  (for _array_element CustomerTheoreticalCheckList ; Foreach vegetable, check if it's available in the level. If so, add to definitive checklist
    (bind _result (Utilities|CheckListContains LevelCheckList _array_element)
      (:Completed
        (if _result
          (Utilities|Array|Add (Variables|Configuration|GetCheckListPossibilities) _array_element))))))