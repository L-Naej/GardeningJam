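; Player controller for a top-down farming game, handling seed pickup, planting, harvesting and delivery to customers.
; It allows one carried item at a time, attached to the character's grab socket, with planting spawning a vegetable of the seed's type.
; A last-clicked-actor gate restricts interactions while carrying.
; Deliveries that match a customer's order raise the PlayerState score, and the controller also creates the HUD widget that shows game over.
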(event EventBeginPlay
  (Utilities|FlowControl|DoOnce false
    (:Completed
      (bind _returnvalue (UserInterface|CreateWidget "/Game/UI/UI_Vegetables.UI_Vegetables_C" self))
      (bind _output_get (Variables|Default|SetPlayerInterface _returnvalue))
      (UserInterface|Viewport|AddtoViewport _output_get 0))))

(event EventOnReset
  (Variables|Internal|SetCurrentlyCarriedSeed 0)
  (Variables|Internal|SetLastActorClicked 0)
  (Variables|Default|SetbIsCarryingVegetable false))

(fn ConstructionScript)

(fn PickSeed
  (params (Vegetable :type Actor%20Object%20Reference))
  (Variables|Internal|GetCurrentlyCarriedSeed ; Currently we want to be able to pick only one seed at a time
    (:then)
    (:else
      (if (Utilities|IsValid Vegetable)
        (bind _asbp_harvest_moon_player_state (Utilities|Casting|CastToBP_HarvestMoonPlayerState (Variables|Default|GetPlayerState)))
        (Default|AddSeedtoInventory _asbp_harvest_moon_player_state Vegetable)
        (bind _astop_down_character (Utilities|Casting|CastToTopDownCharacter (Pawn|GetControlledPawn)))
        (Transformation|AttachComponentToComponent Vegetable (Variables|/Script/Engine.Character|GetMesh _astop_down_character) "Grab_Socket" "SnapToTarget" "SnapToTarget" "KeepWorld" false)
        (Actor|SetOwner Vegetable self)
        (Default|MarkasCarryingSeeds _astop_down_character)
        (bind _output_get (Variables|Internal|SetCurrentlyCarriedSeed Vegetable))
        ;[1 1 1] We dont wan't the seed to block the player input!
        (bind _asbp_seed (Utilities|Casting|CastToBP_Seed _output_get))
        (Collision|SetCollisionResponsetoChannel (Variables|/Game/Gameplay/BP_Interactable.BP_Interactable_C|GetStaticMesh _asbp_seed) "ECC_Visibility" "ECR_Ignore")))))

(fn PlantSeed
  (params (PlantTransform :type Transform))
  (if (Utilities|IsValid (Variables|Internal|GetCurrentlyCarriedSeed))
    (bind _asbp_seed (Utilities|Casting|CastToBP_Seed (Variables|Internal|GetCurrentlyCarriedSeed)))
    (bind _returnvalue (Game|SpawnActorfromClass "/Game/Gameplay/Vegetables/BP_Vegetable.BP_Vegetable_C" PlantTransform "AlwaysSpawn" 0 (Variables|/Game/Gameplay/Vegetables/BP_Seed.BP_Seed_C|GetSeedType _asbp_seed) 0))
    (Default|Plant _returnvalue)
    (bind _astop_down_character (Utilities|Casting|CastToTopDownCharacter (Pawn|GetControlledPawn)))
    (Default|MarkasNotCarryingSeeds _astop_down_character)
    (Actor|DestroyActor (Variables|Internal|GetCurrentlyCarriedSeed))
    (Variables|Internal|SetCurrentlyCarriedSeed 0)))

(fn GetNbSeeds
  (bind _asbp_harvest_moon_player_state (Utilities|Casting|CastToBP_HarvestMoonPlayerState (Variables|Default|GetPlayerState)))
  (bind _nbseeds (Default|GetNbSeeds _asbp_harvest_moon_player_state))
  (return _nbseeds))

(fn ActivateGameOver
  (params (bHasPlayerWon :type Boolean))
  (bind _asui_vegetables (Utilities|Casting|CastToUI_Vegetables (Variables|Default|GetPlayerInterface)))
  (Default|ShowGameOver _asui_vegetables bHasPlayerWon))

(fn TrytoRegisterasLastActorClicked
  (params (ActorClicked :type Actor%20Object%20Reference))
  ;[1 1 1] You cannot register if the player is already in the middle of an action (carrying a seed or a vegetable). Except if you are a customer
  (if (or (not (or (and (Utilities|IsValid (Variables|Internal|GetCurrentlyCarriedSeed)) (not (== (Utilities|GetClass ActorClicked) "/Game/Gameplay/Fields/BP_FieldColumn.BP_FieldColumn_C"))) (Variables|Default|GetbIsCarryingVegetable))) (== (Utilities|GetClass ActorClicked) "/Game/Gameplay/Orders/Customers/BP_Customer_Base.BP_Customer_Base_C"))
    (Variables|Internal|SetLastActorClicked ActorClicked)))

(fn OverlappedActorIsLastActorClicked
  (params (OverlappedActor :type Actor%20Object%20Reference))
  (return (== OverlappedActor (Variables|Internal|GetLastActorClicked))))

(fn HarvestVegetable
  (params (Vegetable :type Actor%20Object%20Reference))
  (if (and (not (Utilities|IsValid (Variables|Internal|GetCurrentlyCarriedSeed))) (not (Variables|Default|GetbIsCarryingVegetable)))
    (Actor|SetOwner Vegetable self)
    (Variables|Default|SetbIsCarryingVegetable true)
    (bind _astop_down_character (Utilities|Casting|CastToTopDownCharacter (Pawn|GetControlledPawn)))
    (Transformation|AttachComponentToComponent Vegetable (Variables|/Script/Engine.Character|GetMesh _astop_down_character) "Grab_Socket" "SnapToTarget" "SnapToTarget" "KeepWorld" false)
    (Variables|Internal|SetCurrentlyCarriedVegetable Vegetable)))

(fn DeliverCarriedVegetable
  (params (CustomerToDeliver :type BP%20Customer%20Base%20Object%20Reference))
  (if (Variables|Default|GetbIsCarryingVegetable)
    (bind _asbp_vegetable (Utilities|Casting|CastToBP_Vegetable (Variables|Internal|GetCurrentlyCarriedVegetable)))
    (bind _output_get (LocalVariables|SetVegetableType (Variables|/Game/Gameplay/Vegetables/BP_Vegetable.BP_Vegetable_C|GetType _asbp_vegetable)))
    ;[1 1 1] Check if the customer is actually one wanting the vegetable we have. If not, abort.
    (bind _success (Default|GiveOrderPart CustomerToDeliver _output_get))
    (if _success
      ;[1 1 1] Destroy carried vegetable if any
      (Actor|DestroyActor (Variables|Internal|GetCurrentlyCarriedVegetable))
      (Variables|Internal|SetCurrentlyCarriedVegetable 0)
      (Variables|Default|SetbIsCarryingVegetable false)
      ;[1 1 1] Increment score
      (bind _asbp_harvest_moon_player_state (Utilities|Casting|CastToBP_HarvestMoonPlayerState (Variables|/Script/Engine.Controller|GetPlayerState (Game|GetPlayerController 0))))
      (Default|IncrementScore _asbp_harvest_moon_player_state)
      (Default|CallOnScoreUpdate (Variables|/Game/Gameplay/Player/BP_HarvestMoonPlayerState.BP_HarvestMoonPlayerState_C|GetPlayerScore _asbp_harvest_moon_player_state)))))