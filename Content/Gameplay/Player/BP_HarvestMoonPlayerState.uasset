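; Player state Blueprint for Harvest Moon that tracks a player's seed inventory and score.
; Inventory is a plain counter: add and remove functions adjust it by one, ignoring the vegetable passed in, with no lower bound on removal.
; Query functions report the seed count and whether any remain, while a separate function increments the score.
; The reset event zeroes both inventory and score.
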(event EventBeginPlay)

(event EventTick
  (params (DeltaSeconds :type Float%20%28single-precision%29)))

(event EventOnReset
  (Variables|Default|SetInventory 0)
  (Variables|Default|SetPlayerScore 0))

(fn ConstructionScript)

(fn AddSeedtoInventory
  (params (NewVegetable :type Actor%20Object%20Reference))
  (Math|Integer|IncrementInt (Variables|Default|GetInventory)))

(fn RemoveSeedfromInventory
  (params (VegetableToRemove :type Actor%20Object%20Reference))
  (Math|Integer|DecrementInt (Variables|Default|GetInventory)))

(fn HasSeedsinInventory
  (return (> (Variables|Default|GetInventory) 0)))

(fn GetNbSeeds
  (return (Variables|Default|GetInventory)))

(fn IncrementScore
  (Math|Integer|IncrementInt (Variables|Default|GetPlayerScore)))