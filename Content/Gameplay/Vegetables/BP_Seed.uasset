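; BP_Seed is an interactable vegetable seed that the player can pick up.
; The construction script colors its mesh by SeedType: pumpkin, cabbage or tomato.
; On interact, it passes itself to PickSeed on the BP_HarvestMoonPlayerController.
; On reset or level reset, it destroys itself only if its owner is a PlayerController, meaning the player is holding it.
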(event EventOnResetLevel
  ;[1 1 1] If resetted while being posessed by player: destroy.
  (Utilities|Casting|CastToPlayerController (Components|GetOwner))
  (Actor|DestroyActor))

(event EventOnInteract
  (bind _asbp_harvest_moon_player_controller (Utilities|Casting|CastToBP_HarvestMoonPlayerController (Game|GetPlayerController 0)))
  (Default|PickSeed _asbp_harvest_moon_player_controller self))

(event EventOnReset
  ;[1 1 1] If resetted while being posessed by player: destroy.
  (Utilities|Casting|CastToPlayerController (Components|GetOwner))
  (Actor|DestroyActor))

(fn ConstructionScript
  (|CallParentFunction)
  (switch Utilities|FlowControl|Switch|SwitchonE_VegetableType (Variables|Default|GetSeedType)
    (:NewEnumerator0
      (Rendering|Material|SetMaterial (Variables|Default|GetStaticMesh) 0 "/Game/Geometry/Meshes/MI_CubeOrange.MI_CubeOrange"))
    (:NewEnumerator1
      (Rendering|Material|SetMaterial (Variables|Default|GetStaticMesh) 0 "/Game/Geometry/Meshes/MI_CubeGreen.MI_CubeGreen"))
    (:NewEnumerator2
      (Rendering|Material|SetMaterial (Variables|Default|GetStaticMesh) 0 "/Game/Geometry/Meshes/MI_CubeBlue.MI_CubeBlue"))))