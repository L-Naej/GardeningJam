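; BP_SeedsSpawner keeps seeds stocked at three spawn points, placing a BP_Seed at each on BeginPlay.
; When an overlap ends at a spawn point, a one-shot timer is stored for that point and spawns a replacement after a configurable delay.
; On reset or level reset, any point with a pending timer respawns its seed immediately and clears that timer.
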(event OnComponentEndOverlap(Spawn1)
  (params (OverlappedComponent :type Primitive%20Component%20Object%20Reference) (OtherActor :type Actor%20Object%20Reference) (OtherComp :type Primitive%20Component%20Object%20Reference) (OtherBodyIndex :type Integer))
  (bind _returnvalue (Utilities|Time|SetTimerbyEvent (delegate Custom|Respawn1) (Variables|Default|GetRespawnTimeInSeconds)))
  (Variables|Default|SetTimer1 _returnvalue))

(event OnComponentEndOverlap(Spawn2)
  (params (OverlappedComponent :type Primitive%20Component%20Object%20Reference) (OtherActor :type Actor%20Object%20Reference) (OtherComp :type Primitive%20Component%20Object%20Reference) (OtherBodyIndex :type Integer))
  (bind _returnvalue (Utilities|Time|SetTimerbyEvent (delegate Custom|Respawn2) (Variables|Default|GetRespawnTimeInSeconds)))
  (Variables|Default|SetTimer2 _returnvalue))

(event OnComponentEndOverlap(Spawn3)
  (params (OverlappedComponent :type Primitive%20Component%20Object%20Reference) (OtherActor :type Actor%20Object%20Reference) (OtherComp :type Primitive%20Component%20Object%20Reference) (OtherBodyIndex :type Integer))
  (bind _returnvalue (Utilities|Time|SetTimerbyEvent (delegate Custom|Respawn3) (Variables|Default|GetRespawnTimeInSeconds)))
  (Variables|Default|SetTimer3 _returnvalue))

(event Custom|Respawn2
  (CallFunction|SpawnSeed (Variables|Default|GetSpawn2)))

(event Custom|Respawn1
  (CallFunction|SpawnSeed (Variables|Default|GetSpawn1)))

(event Custom|Respawn3
  (CallFunction|SpawnSeed (Variables|Default|GetSpawn3)))

(event EventBeginPlay
  (Utilities|FlowControl|Sequence
    (:then_0
      (CallFunction|SpawnSeed (Variables|Default|GetSpawn1)))
    (:then_1
      (CallFunction|SpawnSeed (Variables|Default|GetSpawn2)))
    (:then_2
      (CallFunction|SpawnSeed (Variables|Default|GetSpawn3)))))

(event EventOnResetLevel
  (CallFunction|CheckifShouldRespawnonReset (Variables|Default|GetSpawn1) (Variables|Default|GetTimer1))
  (CallFunction|CheckifShouldRespawnonReset (Variables|Default|GetSpawn2) (Variables|Default|GetTimer2))
  (CallFunction|CheckifShouldRespawnonReset (Variables|Default|GetSpawn3) (Variables|Default|GetTimer3)))

(event EventOnReset
  (CallFunction|CheckifShouldRespawnonReset (Variables|Default|GetSpawn1) (Variables|Default|GetTimer1))
  (CallFunction|CheckifShouldRespawnonReset (Variables|Default|GetSpawn2) (Variables|Default|GetTimer2))
  (CallFunction|CheckifShouldRespawnonReset (Variables|Default|GetSpawn3) (Variables|Default|GetTimer3)))

(fn ConstructionScript)

(fn SpawnSeed
  (params (SeedSpawnPoint :type Scene%20Component%20Object%20Reference))
  (Game|SpawnActorfromClass "/Game/Gameplay/Vegetables/BP_Seed.BP_Seed_C" (Math|Transform|MakeTransform (Transformation|GetWorldLocation SeedSpawnPoint) "0, 0, 0" "1,1,1") "Undefined" 0 "NewEnumerator0" 0))

(fn CheckifShouldRespawnonReset
  (params (SeedSpawnPoint :type Scene%20Component%20Object%20Reference) (Timer :type Timer%20Handle%20Structure))
  (if (Class|KismetSystemLibrary|TimerExistsHandle Timer)
    (CallFunction|SpawnSeed SeedSpawnPoint)
    (Utilities|Time|ClearandInvalidateTimerbyHandle Timer)))