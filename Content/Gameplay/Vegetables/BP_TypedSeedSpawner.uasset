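; BP_TypedSeedSpawner keeps a spawn point stocked with a BP_Seed of its configured SeedType.
; It spawns a seed on BeginPlay, and any end overlap on the Spawn1 component starts a one-shot timer that spawns a replacement after RespawnTimeInSeconds.
; On reset, an existing respawn timer is cleared and its seed spawns immediately.
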(event OnComponentEndOverlap(Spawn1)
  (params (OverlappedComponent :type Primitive%20Component%20Object%20Reference) (OtherActor :type Actor%20Object%20Reference) (OtherComp :type Primitive%20Component%20Object%20Reference) (OtherBodyIndex :type Integer))
  (bind _returnvalue (Utilities|Time|SetTimerbyEvent (delegate Custom|Respawn1) (Variables|Configuration|GetRespawnTimeInSeconds)))
  (Variables|Internal|SetTimer1 _returnvalue))

(event Custom|Respawn1
  (CallFunction|SpawnSeed (Variables|Default|GetSpawn1)))

(event EventBeginPlay
  (CallFunction|SpawnSeed (Variables|Default|GetSpawn1)))

(event EventOnReset
  (CallFunction|CheckifShouldRespawnonReset (Variables|Default|GetSpawn1) (Variables|Internal|GetTimer1)))

(fn ConstructionScript)

(fn SpawnSeed
  (params (SeedSpawnPoint :type Scene%20Component%20Object%20Reference))
  (Game|SpawnActorfromClass "/Game/Gameplay/Vegetables/BP_Seed.BP_Seed_C" (Math|Transform|MakeTransform (Transformation|GetWorldLocation SeedSpawnPoint) "0, 0, 0" "1,1,1") "Undefined" 0 (Variables|Configuration|GetSeedType) 0))

(fn CheckifShouldRespawnonReset
  (params (SeedSpawnPoint :type Scene%20Component%20Object%20Reference) (Timer :type Timer%20Handle%20Structure))
  (if (Class|KismetSystemLibrary|TimerExistsHandle Timer)
    (CallFunction|SpawnSeed SeedSpawnPoint)
    (Utilities|Time|ClearandInvalidateTimerbyHandle Timer)))