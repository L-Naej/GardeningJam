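; Plantable crop actor that grows, becomes harvestable, then decays unless harvested in time.
; BeginPlay loads timings and price from a data table row named by its type enum, while timers drive growth stages shown through dynamic material color.
; Interacting harvests ripe crops via the player controller or starts a weeding countdown on decayed ones, cancelled when the player leaves the sphere.
; Completed weeding or a reset event destroys the actor.
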(event OnComponentEndOverlap(Sphere)
  (params (OverlappedComponent :type Primitive%20Component%20Object%20Reference) (OtherActor :type Actor%20Object%20Reference) (OtherComp :type Primitive%20Component%20Object%20Reference) (OtherBodyIndex :type Integer))
  ;[1 1 1] If player goes far away from the vegetable while weeding, the weeding stops
  (Utilities|Casting|CastToTopDownCharacter OtherActor)
  (if (Utilities|Time|IsValidTimerHandle (Variables|Internal|GetWeedTimer))
    (Utilities|Time|ClearandInvalidateTimerbyHandle (Variables|Internal|GetWeedTimer))
    (Development|SetHiddeninGame (Variables|Default|GetWeedTimerIndicator) true false)
    (Variables|Internal|SetWeedTimerCounter (Variables|Configuration|GetWeedTimeInSeconds))
    (Utilities|Time|ClearandInvalidateTimerbyHandle (Variables|Internal|GetWeedTimerIndicatorHandle))))

(event Custom|OnWeedFinished
  (Rendering|SetActorHiddenInGame true)
  (Actor|DestroyActor))

(event Custom|UpdateWeeTimerIndicator
  (bind _output_get (Variables|Internal|SetWeedTimerCounter (- (Variables|Internal|GetWeedTimerCounter) (Variables|Configuration|GetWeedTimerIndicatorRefreshRateInSeconds))))
  (Rendering|Components|TextRender|SetText (Variables|Default|GetWeedTimerIndicator) (Utilities|Text|ToText(Float) _output_get "HalfToEven")))

(event EventBeginPlay
  (CallFunction|Init))

(event EventOnInteract
  (if (and (Variables|Default|GetbIsReadyToBeHarvested) (not (Variables|Default|GetbIsDecayed)))
    (bind _asbp_harvest_moon_player_controller (Utilities|Casting|CastToBP_HarvestMoonPlayerController (Game|GetPlayerController 0)))
    (Default|HarvestVegetable _asbp_harvest_moon_player_controller self)
    (Utilities|Time|ClearandInvalidateTimerbyHandle (Variables|Internal|GetDecayTimer))
    (elif (Variables|Default|GetbIsDecayed)
      (bind _returnvalue (Utilities|Time|SetTimerbyEvent (delegate Custom|OnWeedFinished) (Variables|Configuration|GetWeedTimeInSeconds)))
      (Variables|Internal|SetWeedTimer _returnvalue)
      (Development|SetHiddeninGame (Variables|Default|GetWeedTimerIndicator) false false)
      (bind _returnvalue_2 (Utilities|Time|SetTimerbyEvent (delegate Custom|UpdateWeeTimerIndicator) (Variables|Configuration|GetWeedTimerIndicatorRefreshRateInSeconds) true))
      (Variables|Internal|SetWeedTimerIndicatorHandle _returnvalue_2))))

(event EventOnReset
  ;[1 1 1] VEGETABLES NEVER RESET!! (sorry)
  (Actor|DestroyActor))

(fn ConstructionScript
  (|CallParentFunction)
  (bind _returnvalue (Rendering|Material|CreateDynamicMaterialInstance (Rendering|Material|GetMaterial (Variables|Default|GetStaticMesh) 0) "None" :!class /Script/Engine.KismetMaterialLibrary))
  (bind _output_get (Variables|Internal|SetMI_Status _returnvalue))
  (Rendering|Material|SetMaterial (Variables|Default|GetStaticMesh) 0 _output_get)
  (Rendering|Components|TextRender|SetText (Variables|Default|GetWeedTimerIndicator) (Utilities|Text|ToText(Float) (Variables|Configuration|GetWeedTimeInSeconds) "HalfToEven"))
  (Variables|Internal|SetWeedTimerCounter (Variables|Configuration|GetWeedTimeInSeconds))
  (switch Utilities|FlowControl|Switch|SwitchonE_VegetableType (Variables|Configuration|GetType)
    (:NewEnumerator0
      (Variables|Configuration|SetReadyToBeHarvestedColor "(R=1.000000,G=0.212760,B=0.000000,A=1.000000)"))
    (:NewEnumerator1
      (Variables|Configuration|SetReadyToBeHarvestedColor "(R=0.284255,G=1.000000,B=0.136735,A=1.000000)"))
    (:NewEnumerator2
      (Variables|Configuration|SetReadyToBeHarvestedColor "(R=0.000000,G=0.100000,B=1.000000,A=1.000000)"))))

(fn OnReadytobeHarvested
  (Rendering|Material|SetVectorParameterValue (Variables|Internal|GetMI_Status) "Color" (Variables|Configuration|GetReadyToBeHarvestedColor) :!class /Script/Engine.MaterialInstanceDynamic)
  (Variables|Default|SetbIsReadyToBeHarvested true)
  (bind _returnvalue (Utilities|Time|SetTimerbyFunctionName self "OnVegetableDecayed" (Variables|Configuration|GetDecayTimeInSeconds)))
  (Variables|Internal|SetDecayTimer _returnvalue))

(fn Plant
  (Utilities|Time|SetTimerbyFunctionName self "OnReadyToBeHarvested" (Variables|Configuration|GetGrowingTimeInSeconds))
  (Variables|Default|SetbIsPlanted true))

(fn OnVegetableDecayed
  (Rendering|Material|SetVectorParameterValue (Variables|Internal|GetMI_Status) "Color" (Variables|Configuration|GetIsDecayedColor) :!class /Script/Engine.MaterialInstanceDynamic)
  (Variables|Default|SetbIsDecayed true))

(fn Init
  (bind _type (Variables|Configuration|GetType))
  (bind _returnvalue (Utilities|String|EnumtoString _type))
  ;[1 1 1] Init vegetable date from data table.
  (bind _returnvalue_2 (Utilities|GetDataTableRow (Variables|Internal|GetVegetablesDataAsset) (Utilities|String|StringToName _returnvalue))
    (:then
      (if (Utilities|Enum|Equal(Enum) (.Type (Utilities|Struct|BreakVegetableData _returnvalue_2)) (Variables|Configuration|GetType)) ; Safety check
        (Variables|Configuration|SetGrowingTimeInSeconds (.GrowthTimeInSeconds (Utilities|Struct|BreakVegetableData _returnvalue_2)))
        (Variables|Configuration|SetDecayTimeInSeconds (.DecayTimeInSeconds (Utilities|Struct|BreakVegetableData _returnvalue_2)))
        (Variables|Configuration|SetPrice (.Price (Utilities|Struct|BreakVegetableData _returnvalue_2)))
        (else
          (Development|PrintString "Warning: Vegetable data row found not coherent with vegetable actual type."))))
    (:RowNotFound
      (Development|PrintString (Utilities|String|Append "Vegetable data row not found, row name not found: " _returnvalue)))))